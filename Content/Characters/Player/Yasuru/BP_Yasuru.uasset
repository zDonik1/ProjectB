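; BP_Yasuru is a player character Blueprint that turns attack overlap checks into Gameplay Ability System events.
; InitiateAttackCheck gathers BP_Enemy actors overlapping the AttackCollider, skipping itself.
; For each hit it sends an Ability.BasicAttack gameplay event to itself, passing itself as instigator and the enemy as target and target data.
; The construction script only calls its parent.
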(event `InitiateAttackCheck`
  (for _array_element (`PrimitiveComponent.GetOverlappingActors` (`self.AttackCollider`) "/Game/Characters/Enemy/BP_Enemy.BP_Enemy_C")
    (if (!= _array_element self)
      (`AbilitySystemBlueprintLibrary.SendGameplayEventToActor` self (struct :`TagName` "Ability.BasicAttack") (make `GameplayEventData` (struct) self _array_element null null (struct) (struct) (struct) 0.0 (`AbilitySystemBlueprintLibrary.AbilityTargetDataFromActor` _array_element))))))

(fn `UserConstructionScript`
  (`parent.UserConstructionScript`))