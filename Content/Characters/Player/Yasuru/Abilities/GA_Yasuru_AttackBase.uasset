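; Gameplay ability for Yasuru's base attack, turning the character toward move input or forward and playing an attack montage.
; The montage's play rate is scaled so it fits the configured attack duration.
; A one-shot wait for the Ability.BasicAttack gameplay event applies damage from the event's target data.
; An attack tag is held until montage blend-out, which also cancels the wait and ends the ability.
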(event `self.K2_ActivateAbility`
  (`parent.K2_ActivateAbility`)
  (`self.K2_CommitAbility`)
  (`self.PerformAttack`))

(event `PerformAttack`
  (bind _attackmontage (`self.AttackMontage`))
  (`PBAbilitySystemComponent.AddTag` (`self.AbilitySystemComp`) (`self.AttackTag`))
  (`Actor.K2_SetActorRotation` (`self.Character`) (`KismetMathLibrary.Conv_VectorToRotator` (`/Game/Characters/Player/BP_PlayerController.GetMoveOrForwardVector` (`self.PlayerController`))) false)
  (bind _returnvalue (`AnimSequenceBase.GetPlayLength` _attackmontage))
  (`|PlayMontage` (`self.SkeletalMeshComponent`) _attackmontage (/ _returnvalue (`self.AttackDuration`))
    (:`then`
      (bind (_asynctaskproxy _payload) (`AbilityTask_WaitGameplayEvent.WaitGameplayEvent` (struct :`TagName` "Ability.BasicAttack") null true)
        (:`EventReceived`
          (`self.ApplyDamageFromEvent` (`.TargetData` (break `GameplayEventData` _payload))))))
    (:`OnBlendOut`
      (`PBAbilitySystemComponent.RemoveTag` (`self.AbilitySystemComp`) (`self.AttackTag`))
      (`/Engine/EditorBlueprintResources/StandardMacros.IsValid` _asynctaskproxy
        (:`Is Valid`
          (`GameplayTask.EndTask` _asynctaskproxy))
        (:`Is Not Valid`
          _))
      (`self.K2_EndAbility`))))