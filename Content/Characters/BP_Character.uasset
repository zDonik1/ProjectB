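; BP_Character is a character with an Ability System health attribute, an overhead health bar widget, hit reactions and death.
; BeginPlay links the widget to its owner and binds health changes, which set the bar's percent from the attribute ratio.
; OnHIt checks health, either playing a hit-react montage with movement disabled until completion or calling OnDeath.
; Death flags the Anim Blueprint, disables capsule collision and tick, unpossesses, and hides the bar.
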(event `self.ReceiveBeginPlay`
  ;[1 1 1] Setting up HealthBar
  (bind _asbpui_health_bar (cast `/Game/Blueprints/BPUI_HealthBar` (`WidgetComponent.GetUserWidgetObject` (`self.HealthBarComponent`))))
  (bind _output_get (set `self.HealthBarWidget` _asbpui_health_bar))
  (set `/Game/Blueprints/BPUI_HealthBar.OwningCharacter` self _output_get)
  (add `self.OnHealthChange` (delegate `OnHealthUpdated`))
  (bind _asabp_character (cast `/Game/Mannequin/Animations/ABP_Character` (`SkeletalMeshComponent.GetAnimInstance` (`self.Mesh`))))
  (set `self.AnimInstance` _asabp_character))

(event `OnHealthUpdated` :!signature `self.OnHealthChange`
  (params (AttributeValue :type "Float (double-precision)"))
  ;[1 1 1] Update Health Bar
  (`ProgressBar.SetPercent` (`/Game/Blueprints/BPUI_HealthBar.HealthBar` (`self.HealthBarWidget`)) (/ AttributeValue (`.ReturnValue` (`AbilitySystemBlueprintLibrary.GetFloatAttributeBaseFromAbilitySystemComponent` (`self.AbilitySystemComponent`) (struct :`AttributeName` "MaxHealth" :`Attribute` "/Script/ProjectB.PBHealthAttributeSet:MaxHealth"))))))

(event `OnDeath`
  ;[1 1 1] Hit Events
  (bind _asabp_character (cast `/Game/Mannequin/Animations/ABP_Character` (`SkeletalMeshComponent.GetAnimInstance` (`self.Mesh`))))
  (set `/Game/Mannequin/Animations/ABP_Character.IsDead` true _asabp_character)
  (`PrimitiveComponent.SetCollisionEnabled` (`self.CapsuleComponent`) "NoCollision")
  (`self.SetActorTickEnabled` false)
  (`Controller.UnPossess` (`self.GetController`))
  (`SceneComponent.SetVisibility` (`self.HealthBarComponent`) false false))

(event `OnHIt`
  (bind _charactermovement (`self.CharacterMovement`))
  ;[1 1 1] Hit Events
  (if (<= (`.ReturnValue` (`AbilitySystemBlueprintLibrary.GetFloatAttributeBaseFromAbilitySystemComponent` (`self.AbilitySystemComponent`) (struct :`AttributeName` "Health" :`Attribute` "/Script/ProjectB.PBHealthAttributeSet:Health"))) 0.0)
    (`self.OnDeath`)
    (else
      (`|PlayMontage` (`self.Mesh`) "/Game/Mannequin/Animations/AM_HitReact.AM_HitReact"
        (:`then`
          (`CharacterMovementComponent.DisableMovement` _charactermovement))
        (:`OnCompleted`
          (`CharacterMovementComponent.SetMovementMode` _charactermovement "MOVE_Walking" 0))))))

(fn `UserConstructionScript`)