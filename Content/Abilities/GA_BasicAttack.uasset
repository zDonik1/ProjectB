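; GA_BasicAttack is a controller ability for a two-hit basic attack combo, granting GA_Attack1 and GA_Attack2 and starting Attack1 on activation.
; A click-counting macro with a one-second delay detects double presses, which queue Attack2 during Attack1 or fire it immediately otherwise.
; Gameplay tag removal drives the chain: Attack1 ending releases the queued Attack2, and Attack2 ending, like a single click, ends the ability.
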(event `self.BlueprintInitInstance`
  (bind _character (`self.Character`))
  (`parent.BlueprintInitInstance`)
  (`PBCharacter.GrantAbility` _character "/Game/Abilities/Secondary/GA_Attack1.GA_Attack1_C")
  (`PBCharacter.GrantAbility` _character "/Game/Abilities/Secondary/GA_Attack2.GA_Attack2_C")
  (add `PBAbilitySystemComponent.OnTagChanged` (`self.AbilitySystemComp`) (delegate `OnTagChanged`)))

(event `OnTagChanged`
  (params (Tag :type "GameplayTag Structure") (Exists :type Boolean))
  (`self.HandleTagChanged` Tag Exists))

(event `self.K2_ActivateAbility`
  (`parent.K2_ActivateAbility`)
  (set `self.bShouldSecondAttack` false)
  (set `self.bPerformedSecondAttack` false)
  (`AbilitySystemComponent.TryActivateAbilityByClass` (`self.AbilitySystemComp`) "/Game/Abilities/Secondary/GA_Attack1.GA_Attack1_C" true))

(event `self.K2_OnEndAbility`
  (params (bWasCancelled :type Boolean))
  (goto _label :!via `Reset`))

(event `self.BlueprintInputPressed`
  (`self.HasDoubleClicked` :!label _label
    (:`Double`
      (bind _returnvalue (`PBAbilitySystemComponent.HasActiveAbilityWithTag` (`self.AbilitySystemComp`) (struct :`TagName` "Ability.BasicAttack.Attack1")))
      (if _returnvalue
        (set `self.bShouldSecondAttack` true)
        (else
          (`self.TryPerformSecondAttack`))))
    (:`Single`
      (`self.K2_EndAbility`))))

(event `HandleTagChanged`
  (params (Tag :type "GameplayTag Structure") (Exists :type Boolean))
  (if (not Exists)
    (`|SwitchGameplayTag` Tag
      (:`Ability.BasicAttack.Attack1`
        (if (`self.bShouldSecondAttack`)
          (`self.TryPerformSecondAttack`)))
      (:`Ability.BasicAttack.Attack2`
        (`self.K2_EndAbility`)))))

(fn `TryPerformSecondAttack`
  (if (not (`self.bPerformedSecondAttack`))
    (`AbilitySystemComponent.TryActivateAbilityByClass` (`self.AbilitySystemComp`) "/Game/Abilities/Secondary/GA_Attack2.GA_Attack2_C" true)
    (set `self.bPerformedSecondAttack` true)))