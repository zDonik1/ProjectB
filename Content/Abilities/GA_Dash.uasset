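; Dash gameplay ability that sends the character a set distance toward movement input or facing, damaging enemies it passes through.
; It locks move input, sets the capsule to overlap pawns, plays a duration-scaled wind-up montage, then runs a root-motion MoveTo task.
; An overlap/hit task damages "Enemy" actors, while a blocking hit stops the dash at the impact location.
; Finishing restores pawn blocking, waits out recovery, then returns input.
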(event `self.K2_ActivateAbility`
  (bind _dashwindupmontage (`self.DashWindUpMontage`))
  (bind _returnvalue (`/Game/Characters/Player/BP_PlayerController.GetMoveOrForwardVector` (`self.PlayerController`)))
  (`parent.K2_ActivateAbility`)
  (`self.K2_CommitAbility`)
  (set `self.DashDirection` (`KismetMathLibrary.Vector_NormalUnsafe` _returnvalue))
  (`Actor.K2_SetActorRotation` (`self.Character`) (`KismetMathLibrary.Conv_VectorToRotator` _returnvalue) false)
  (`Controller.SetIgnoreMoveInput` (`self.PlayerController`) true)
  (`PrimitiveComponent.SetCollisionResponseToChannel` (`Character.CapsuleComponent` (`self.Character`)) "ECC_Pawn" "ECR_Overlap")
  (bind _returnvalue_2 (`AnimSequenceBase.GetPlayLength` _dashwindupmontage))
  (`|PlayMontage` (`self.SkeletalMeshComponent`) _dashwindupmontage (/ _returnvalue_2 (`self.WindUpDuration`))
    (:`OnBlendOut`
      (set `/Game/Mannequin/Animations/ABP_Character.bIsDashing` true (`self.AnimInstance`))
      (bind _asynctaskproxy (`AbilityTask_ApplyRootMotionMoveToForce.ApplyRootMotionMoveToForce` "None" (+ (`Actor.K2_GetActorLocation` (`self.Character`)) (* (`self.DashDirection`) (`self.DashDistance`))) (/ (`self.DashDistance`) (`self.DashSpeed`)) false "MOVE_None" true null "SetVelocity")
        (:`then`
          (bind (_asynctaskproxy_2 _targetdata) (`PBAbilityTask_WaitOverlapHit.WaitForOverlapHit`)
            (:`OnOverlap`
              (bind (_bblockinghit _binitialoverlap _time _distance _location _impactpoint _normal _impactnormal _physmat _hitactor) (`GameplayStatics.BreakHitResult` (`AbilitySystemBlueprintLibrary.GetHitResultFromTargetData` _targetdata)))
              (if (`Actor.ActorHasTag` _hitactor "Enemy")
                (`self.ApplyDamageFromEvent` _targetdata)))
            (:`OnHit`
              (`GameplayTask.EndTask` _asynctaskproxy)
              (`Actor.K2_SetActorLocation` (`self.Character`) _location false false) ; Character might jitter after hit so setting location
              (`GameplayTask.EndTask` _asynctaskproxy_2)
              (`PrimitiveComponent.SetCollisionResponseToChannel` (`Character.CapsuleComponent` (`self.Character`)) "ECC_Pawn" "ECR_Block" :!label _label)
              (`KismetSystemLibrary.Delay` (`self.RecoverDuration`))
              (set `/Game/Mannequin/Animations/ABP_Character.bIsDashing` false (`self.AnimInstance`))
              (`Controller.SetIgnoreMoveInput` (`self.PlayerController`) false)
              (`self.K2_EndAbility`))))
        (:`OnTimedOut`
          (goto _label))
        (:`OnTimedOutAndDestinationReached`
          (goto _label))))))

(fn `DisableMoveInput`
  (`CharacterMovementComponent.DisableMovement` (`Character.CharacterMovement` (`self.Character`))))

(fn `EnableMovement`
  (`CharacterMovementComponent.SetMovementMode` (`Character.CharacterMovement` (`self.Character`)) "MOVE_Walking" 0))