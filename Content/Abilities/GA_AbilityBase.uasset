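; GA_AbilityBase is a base Gameplay Ability that caches references to the owning actor's objects, presumably for child abilities to share.
; On instance init, InitReferences reads the actor info to store the character, player controller, anim instance, skeletal mesh and the character's ability system component.
; A failed player controller or anim instance cast calls EndAbility, while a failed character cast has no such handling.
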(event `self.BlueprintInitInstance`
  (bind (_returnvalue_owneractor _returnvalue_avataractor _returnvalue_playercontroller _returnvalue_abilitysystemcomponent _returnvalue_skeletalmeshcomponent) (break `GameplayAbilityActorInfo` (`self.GetActorInfo`)))
  (`|ExecutionSequence`
    (:`then_0`
      (bind _asbp_character (cast `/Game/Characters/BP_Character` _returnvalue_avataractor))
      (set `self.Character` _asbp_character))
    (:`then_1`
      (bind _asbp_player_controller (cast `/Game/Characters/Player/BP_PlayerController` _returnvalue_playercontroller)
        (:`then`
          (set `self.PlayerController` _asbp_player_controller))
        (:`CastFailed`
          (`self.K2_EndAbility` :!label _label))))
    (:`then_2`
      (bind _asabp_character (cast `/Game/Mannequin/Animations/ABP_Character` (`SkeletalMeshComponent.GetAnimInstance` _returnvalue_skeletalmeshcomponent))
        (:`then`
          (set `self.AnimInstance` _asabp_character))
        (:`CastFailed`
          (goto _label))))
    (:`then_3`
      (set `self.SkeletalMeshComponent` _returnvalue_skeletalmeshcomponent))
    (:`then_4`
      (set `self.AbilitySystemComp` (`PBCharacter.AbilitySystemComponent` (`self.Character`))))))