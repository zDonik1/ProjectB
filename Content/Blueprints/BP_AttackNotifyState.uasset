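; Anim notify state that switches a character's sword on for the notify window of an attack animation.
; A helper casts the mesh owner to BP_Character and its ToolActor child actor to BP_BaseSword.
; Notify begin calls Active on that sword and notify end calls Inactive, with no validity check on the result.
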(fn `GetBaseSwordFromMeshComponent`
  (params (`Mesh Component` :type "ActorComponent Object Reference"))
  (returns (`Base Sword` :type "/Game/Weapons/BP_BaseSword Object Reference"))
  (bind _asbp_character (cast `/Game/Characters/BP_Character` (`ActorComponent.GetOwner` `Mesh Component`))
    (:`then`
      (bind _asbp_base_sword (cast `/Game/Weapons/BP_BaseSword` (`ChildActorComponent.ChildActor` (`/Game/Characters/BP_Character.ToolActor` _asbp_character)))
        (:`then`
          _)
        (:`CastFailed`
          _)))
    (:`CastFailed`
      _))
  (return _asbp_base_sword))

(fn `Received_NotifyBegin`
  (params (MeshComp :type "SkeletalMeshComponent Object Reference") (Animation :type "AnimSequenceBase Object Reference") (TotalDuration :type "Float (double-precision)"))
  (returns (ReturnValue :type Boolean))
  (bind _base_sword (`self.GetBaseSwordFromMeshComponent` MeshComp))
  (`/Game/Weapons/BP_BaseSword.Active` _base_sword)
  (return false))

(fn `Received_NotifyEnd`
  (params (MeshComp :type "SkeletalMeshComponent Object Reference") (Animation :type "AnimSequenceBase Object Reference"))
  (returns (ReturnValue :type Boolean))
  (bind _base_sword (`self.GetBaseSwordFromMeshComponent` MeshComp))
  (`/Game/Weapons/BP_BaseSword.Inactive` _base_sword)
  (return true))