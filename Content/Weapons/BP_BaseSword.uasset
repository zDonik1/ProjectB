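; Base sword weapon Blueprint that deals melee damage through a box collider.
; Active and Inactive events switch the collider between query-only and no collision.
; On overlap with an actor other than its owning BP_Character, it applies damage using that character's controller as instigator.
; A DoOnce that resets after a half-second delay throttles hits across all targets.
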(event `self.BoxCollider.OnComponentBeginOverlap`
  (params (OverlappedComponent :type "PrimitiveComponent Object Reference") (OtherActor :type "Actor Object Reference") (OtherComp :type "PrimitiveComponent Object Reference") (OtherBodyIndex :type Integer) (bFromSweep :type Boolean) (SweepResult :type "HitResult Structure (by ref)"))
  (bind _returnvalue (`self.GetOwner`))
  (bind _asbp_character (cast `/Game/Characters/BP_Character` _returnvalue))
  (if (!= OtherActor _returnvalue)
    (`/Engine/EditorBlueprintResources/StandardMacros.DoOnce` false :!label _label
      (:`Completed`
        (`GameplayStatics.ApplyDamage` OtherActor (`self.damage`) (`Pawn.GetController` _asbp_character) self)
        (`KismetSystemLibrary.Delay` 0.5)
        (goto _label :!via `Reset`)))))

(event `Active`
  (`PrimitiveComponent.SetCollisionEnabled` (`self.BoxCollider`) "QueryOnly"))

(event `Inactive`
  (`PrimitiveComponent.SetCollisionEnabled` (`self.BoxCollider`) "NoCollision"))

(fn `UserConstructionScript`)